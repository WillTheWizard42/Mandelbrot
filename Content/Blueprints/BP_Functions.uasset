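; BP_Functions is a set of helper functions for reaching the game mode and the plane material it stores.
; GetGamemode casts the current game mode to BP_Gamemode and returns it with a success flag.
; GetMaterial and SetMaterial read and write PlaneMaterial through that helper without checking the flag, so the game mode acts as the shared store for that material.
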(fn GetGamemode
  (bind _asbp_gamemode (Utilities|Casting|CastToBP_Gamemode (Game|GetGameMode))
    (:then
      (return _asbp_gamemode true))
    (:CastFailed
      (return _asbp_gamemode false))))

(fn GetMaterial
  (return (Variables|/Game/Blueprints/BP_Gamemode.BP_Gamemode_C|GetPlane%20material (.Gamemode (CallFunction|GetGamemode)))))

(fn SetMaterial
  (params (Material :type Material%20Instance%20Dynamic%20Object%20Reference))
  (Variables|/Game/Blueprints/BP_Gamemode.BP_Gamemode_C|SetPlane%20material (.Gamemode (CallFunction|GetGamemode)) Material)
  (return))